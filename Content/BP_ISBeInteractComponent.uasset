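; Blueprint component for the receiving side of an interaction system, handling enter, start, end, leave, complete and attach events from an interact component.
; Each event calls its parent implementation, forwards to a multicast counterpart left empty here, and optionally prints a debug log.
; Helpers read the local player's role sign, check per-trace-type UI display, find a valid target among entered trace types, and branch on network role.
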(event `IS_BeInteractInterface.InteractEnter`
  (params (InteractComponent :type "IS_InteractComponent Object Reference") (TraceType :type "EIS_InteractTraceType Enum" :default "None"))
  (`parent.InteractEnter` InteractComponent TraceType)
  (`self.Multi_InteractEnter` InteractComponent TraceType)
  (`self.Debug` (`KismetStringLibrary.Concat_StrStr` "进入交互" "-" (`|GetEnumeratorNameAsString` TraceType)) InteractComponent))

(event `Multi_InteractEnter`
  (params (InteractComponent :type "IS_InteractComponent Object Reference") (TraceType :type "EIS_InteractTraceType Enum" :default "CameraTrace")))

(event `Multi_InteractStart`
  (params (InteractComponent :type "IS_InteractComponent Object Reference")))

(event `IS_BeInteractInterface.InteractStart`
  (params (InteractComponent :type "IS_InteractComponent Object Reference"))
  (`parent.InteractStart` InteractComponent)
  (`self.Multi_InteractStart` InteractComponent)
  (`self.Debug` "开始交互" InteractComponent))

(event `IS_BeInteractInterface.InteractEnd`
  (params (InteractComponent :type "IS_InteractComponent Object Reference"))
  (`parent.InteractEnd` InteractComponent)
  (`self.Multi_InteractEnd` InteractComponent)
  (`self.Debug` "结束交互" InteractComponent))

(event `Multi_InteractEnd`
  (params (InteractComponent :type "IS_InteractComponent Object Reference")))

(event `IS_BeInteractInterface.InteractLeave`
  (params (InteractComponent :type "IS_InteractComponent Object Reference") (TraceType :type "EIS_InteractTraceType Enum" :default "None"))
  (`parent.InteractLeave` InteractComponent TraceType)
  (`self.Multi_InteractLeave` InteractComponent TraceType)
  (`self.Debug` (`KismetStringLibrary.Concat_StrStr` "离开交互" "-" (`|GetEnumeratorNameAsString` TraceType)) InteractComponent))

(event `Multi_InteractLeave`
  (params (InteractComponent :type "IS_InteractComponent Object Reference") (TraceType :type "EIS_InteractTraceType Enum" :default "CameraTrace")))

(event `IS_BeInteractInterface.InteractComplete`
  (params (InteractComponent :type "IS_InteractComponent Object Reference"))
  (`parent.InteractComplete` InteractComponent)
  (`self.Multi_InteractComplete` null)
  (`self.Debug` "完成交互" InteractComponent))

(event `Multi_InteractComplete`
  (params (InteractComponent :type "IS_InteractComponent Object Reference")))

(event `IS_BeInteractInterface.InteractAttachTo`
  (params (InteractComponent :type "IS_InteractComponent Object Reference"))
  (`parent.InteractAttachTo` InteractComponent)
  (`self.Multi_InteractAttachTo` InteractComponent)
  (`self.Debug` "挂载交互" InteractComponent))

(event `Multi_InteractAttachTo`
  (params (InteractComponent :type "IS_InteractComponent Object Reference")))

(fn `Debug`
  (params (InString :type String) (ISCom :type "IS_InteractComponent Object Reference"))
  (if (`self.IsDebugLog`)
    (`KismetSystemLibrary.PrintString` (`KismetStringLibrary.Concat_StrStr` "IS:" (`KismetSystemLibrary.GetDisplayName` (`self.GetOwner`)) "：" InString "[" (`KismetSystemLibrary.GetDisplayName` (`self.GetOwner` ISCom)) "]"))))

(fn `GetLocalRoleSign`
  (returns (RoleSign :type Name))
  (`self.LocalISCom`
    (:`then`
      _)
    (:`else`
      (set `self.LocalISCom` (`Actor.GetComponentByClass` (`GameplayStatics.GetPlayerPawn` 0) "/Script/InteractSystem.IS_InteractComponent"))))
  (return (`IS_InteractComponent.GetRoleSign` (`self.LocalISCom`))))

(fn `GetValidInteractTargetFromAllType`
  (returns (TopPriorityCom :type "IS_BeInteractComponent Object Reference"))
  (bind _localiscom (`self.LocalISCom`)
    (:`then`
      (bind (_topprioritycom _returnvalue) (`IS_InteractComponent.GetInteractCheckComponentFromType` _localiscom "None"))
      (for _array_element _returnvalue
        (`/Engine/EditorBlueprintResources/StandardMacros.IsValid` _array_element
          (:`Is Valid`
            (bind (_keypin _valuepin) (`|MapForEach` (`.InteractCheckEnterCondition` (break `IS_BeInteractInfo` (`IS_BeInteractComponent.BeInteractInfo` _array_element))))
              (:`then`
                (if (`KismetArrayLibrary.Array_Contains` (`.AllEnterTraceType` (break `IS_BeInteractDynamicInfo` (`IS_BeInteractComponent.BeInteractDynamicInfo` _array_element))) _keypin)
                  (if (`.bIsDisplayInteractUI` (break `IS_BeInteractCheckCondition` _valuepin))
                    (if (`.ReturnValue` (`IS_InteractComponent.InteractConditionCheck` _localiscom _topprioritycom _keypin))
                      (return _array_element))))))))))
    (:`else`
      _))
  (return null))

(fn `IsDisplayInteractUIFromType`
  (params (InteractTraceType :type "EIS_InteractTraceType Enum (by ref)"))
  (returns (ReturnValue :type Boolean))
  (bind (_value _returnvalue) (`BlueprintMapLibrary.Map_Find` (`.InteractCheckEnterCondition` (break `IS_BeInteractInfo` (`self.BeInteractInfo`))) InteractTraceType))
  (if _returnvalue
    (return (`.bIsDisplayInteractUI` (break `IS_BeInteractCheckCondition` _value)))
    (else
      (return false))))