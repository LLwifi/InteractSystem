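; Interactable actor base that animates the actor or its AnimRoot between a start transform and an end transform chosen by interaction angle.
; IS_BeInteractComponent completion triggers a ping-pong timeline that reverses direction each time and lerps the transform.
; When playing forward from the start, the interactor's direction angle is matched against AnimTransformAngle ranges to pick the end offset, composed with the start transform.
; The construction script applies the configured initial start or angle-based pose.
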(event `self.ReceiveBeginPlay`
  (set `self.AnimEndIsReverse` (< (`KismetMathLibrary.Conv_ByteToInt` (`self.InitTransformState`)) 2))
  (set `self.AnimTransform_End` (`self.GetAnimTransformFromAngle` (`self.InitTransformByAngle`)))
  (`self.ISBeInteractCom`
    (:`then`)
    (:`else`
      (set `self.ISBeInteractCom` (`self.GetComponentByClass` "/Script/InteractSystem.IS_BeInteractComponent"))
      (bind _isbeinteractcom (`self.ISBeInteractCom`)
        (:`then`
          (add `IS_BeInteractComponent.OnInteractComplete` _isbeinteractcom (delegate `InteractComplete`)))
        (:`else`)))))

(event `InteractComplete`
  (params (InteractComponent :type "IS_InteractComponent Object Reference") (TraceTypeTag :type "GameplayTag Structure"))
  (`self.PlayAnim_AutoPingPong` (select `bool` (`KismetSystemLibrary.IsValid` InteractComponent) :`true` (`self.K2_GetActorLocation` (`ActorComponent.GetOwner` InteractComponent)))))

(event `PlayAnim`
  (params (IsReverse :type Boolean) (IsFromScratch :type Boolean) (TargetLocation :type "Vector Structure"))
  (bind _returnvalue (== (`self.AnimF`) 0.0))
  (`self.AnimStart`)
  (`TimelineComponent.SetPlayRate` (`self.AnimTimeline`) (/ 1.0 (`self.AnimTime`)))
  (set `self.AnimIsPlaying` true)
  (if IsReverse
    ; 反转播放TimeLine
    (set `self.AnimEndIsReverse` true)
    (if IsFromScratch
      (bind (_direction _f) (`Timeline|AnimTimeline` :!via `ReverseFromEnd` :!label _label)
        (:`Update`
          (`self.AnimUpdate` _f))
        (:`Finished`
          (`self.AnimEnd`)))
      (elif _returnvalue
        (goto _label :!via `Reverse`)
        (else
          (goto _label :!via `Reverse`))))
    (else
      ; 正常播放TimeLine
      (set `self.AnimEndIsReverse` false)
      (if IsFromScratch
        (`self.SetAnimTransformEndFromAngle` TargetLocation)
        (goto _label :!via `PlayFromStart`)
        (elif _returnvalue
          (`self.SetAnimTransformEndFromAngle` TargetLocation)
          (goto _label)
          (else
            (goto _label)))))))

(event `PlayAnim_AutoPingPong`
  (params (TargetLocation :type "Vector Structure"))
  (`self.PlayAnim` (not (`self.AnimEndIsReverse`)) false TargetLocation))

(fn `AnimEnd`
  (set `self.AnimIsPlaying` false))

(fn `AnimStart`)

(fn `AnimUpdate`
  (params (TimelineF :type "Float (double-precision)"))
  (bind _returnvalue (`KismetMathLibrary.TLerp` (`self.AnimTransform_Start`) (`self.AnimTransform_End`) (`self.AnimF`)))
  (set `self.AnimF` TimelineF)
  (if (`self.AnimControlActorOrComponent`)
    (`self.K2_SetActorTransform` _returnvalue)
    (else
      (`SceneComponent.K2_SetRelativeTransform` (`self.AnimRoot`) _returnvalue false false))))

(fn `GetAnimTransformFromAngle`
  (params (Angle :type "Float (double-precision)"))
  (returns (Transform :type "Transform Structure"))
  (locals (LocalVar :type "Transform Structure"))
  (bind _animtransform_angle (`self.AnimTransform_Angle`))
  (bind _angle (`local.Angle`))
  (bind _values (`BlueprintMapLibrary.Map_Values` _animtransform_angle))
  (bind _keys (`BlueprintMapLibrary.Map_Keys` _animtransform_angle))
  (for (_array_element _array_index) _values
    (bind (_lowerbound _upperbound) (break `FloatRange` _array_element))
    (bind (_type _value) (break `FloatRangeBound` _lowerbound))
    (switch `ERangeBoundTypes` _type
      (:`Exclusive`
        (if (> _angle _value)
          (bind (_type_2 _value_2) (break `FloatRangeBound` _upperbound))
          (switch `ERangeBoundTypes` _type_2
            (:`Exclusive`
              (if (< (`local.Angle`) _value_2) :!label _label
                (set `local.LocalVar` (`|GetArrayItem` _keys _array_index) :!label _label_2)
                (break)))
            (:`Inclusive`
              (if (<= (`local.Angle`) _value_2) :!label _label_3
                (goto _label_2)))
            (:`Open`
              (goto _label_2)))))
      (:`Inclusive`
        (if (>= _angle _value)
          (switch `ERangeBoundTypes` _type_2
            (:`Exclusive`
              (goto _label))
            (:`Inclusive`
              (goto _label_3))
            (:`Open`
              (goto _label_2)))))
      (:`Open`
        (switch `ERangeBoundTypes` _type_2
          (:`Exclusive`
            (goto _label))
          (:`Inclusive`
            (goto _label_3))
          (:`Open`
            (goto _label_2))))))
  (return (`/Game/TLBJ/Prototype/Characters/Human/AdvancedLocomotionV4/Blueprints/Libraries/ALS_MacroLibrary.ML_Transform+Transform` (`local.LocalVar`) (`self.AnimTransform_Start`))))

(fn `SetAnimTransformEndFromAngle`
  (params (TargetLocation :type "Vector Structure"))
  (set `self.AnimTransform_End` (`self.GetAnimTransformFromAngle` (`IS_BeInteractComponent.GetAngleFromTargetDir` (`self.ISBeInteractCom`) (- TargetLocation (`self.K2_GetActorLocation`))))))

(fn `UserConstructionScript`
  (bind _animtransform_start (`self.AnimTransform_Start`))
  (bind _animcontrolactororcomponent (`self.AnimControlActorOrComponent`))
  (bind _transform (`self.GetAnimTransformFromAngle` (`self.InitTransformByAngle`)))
  (if (`self.AnimStartIsUseActorTransform`)
    (set `self.AnimTransform_Start` (`self.GetTransform`)))
  (switch `/InteractSystem/BP/E_ISAnimInitStateType` (`self.InitTransformState`)
    (:`NewEnumerator0`
      (if _animcontrolactororcomponent
        (`self.K2_SetActorTransform` _animtransform_start)
        (else
          (`SceneComponent.K2_SetRelativeTransform` (`self.AnimRoot`) _animtransform_start false false))))
    (:`NewEnumerator1`
      (if _animcontrolactororcomponent
        (`self.K2_SetActorTransform` _transform)
        (else
          (`SceneComponent.K2_SetRelativeTransform` (`self.AnimRoot`) _transform false false))))))