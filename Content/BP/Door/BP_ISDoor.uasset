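; Interactable door Blueprint that opens and closes together with an array of linked doors.
; Completing an interaction runs the parent logic, then plays each linked door's animation using the shared reverse state and the interactor owner's location.
; The interact component's collision is disabled during animation.
; Helper functions report open state, check remaining interactions across linked doors, and request state changes through the interaction path only when the state differs.
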(event `self.AnimStart`
  (`parent.AnimStart`)
  (`PrimitiveComponent.SetCollisionEnabled` (`self.ISBeInteractCom`) "NoCollision"))

(event `self.AnimEnd`
  (`parent.AnimEnd`)
  (`PrimitiveComponent.SetCollisionEnabled` (`self.ISBeInteractCom`) "QueryOnly"))

(event `self.InteractComplete`
  (params (InteractComponent :type "IS_InteractComponent Object Reference") (TraceTypeTag :type "GameplayTag Structure"))
  (`parent.InteractComplete` InteractComponent TraceTypeTag)
  (for _array_element (`self.LinkDoor_IsReverse`)
    (`/Engine/EditorBlueprintResources/StandardMacros.IsValid` _array_element
      (:`Is Valid`
        (`self.PlayAnim` _array_element (`self.AnimEndIsReverse`) true (select `bool` (`KismetSystemLibrary.IsValid` InteractComponent) :`true` (`self.K2_GetActorLocation` (`ActorComponent.GetOwner` InteractComponent)))) ; IsReverse为false是开true是关
      ))))

(fn `ChangeDoorState`
  (params (IsOpen :type Boolean) (InteractComponent :type "IS_InteractComponent Object Reference"))
  (if (!= IsOpen (`self.IsOpen`))
    (`self.InteractComplete` InteractComponent)))

(fn `IsOpen`
  (returns (IsOpen :type Boolean))
  (return (not (`self.AnimEndIsReverse`))))

(fn `MyAndLinkDoorIsActive`
  (returns (IsActive :type Boolean))
  (locals (Active :type Boolean :default true))
  ; 自己是否还有交互次数
  (bind _returnvalue (message `IS_BeInteractInterface.IsInteractActive` (`self.ISBeInteractCom`)))
  (if _returnvalue
    ; 链接的其他门是否还有交互次数
    (for _array_element (`self.LinkDoor_IsReverse`)
      (bind _returnvalue_2 (message `IS_BeInteractInterface.IsInteractActive` (`/InteractSystem/BP/BP_ISAnim.ISBeInteractCom` _array_element)))
      (if (not _returnvalue_2)
        (set `local.Active` false)
        (break)))
    (else
      (set `local.Active` false)))
  (return (`local.Active`)))

(fn `UserConstructionScript`)